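; DoorBP is an interactable, lockable door that swings open and closed.
; Interact, ignored while locked, uses a FlipFlop to play or reverse a timeline that lerps the SMDoor mesh yaw to its open angle.
; Each toggle updates IsClose and plays an open or close sound at the world origin.
; LockDoor and UnlockDoor change IsLocked only while the door is flagged closed.
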(event Custom|LockDoor
  (if (Variables|Default|GetisClose)
    (Variables|Default|SetisLocked true)))

(event Custom|UnlockDoor
  (if (Variables|Default|GetisClose)
    (Variables|Default|SetisLocked false)))

(event EventBeginPlay)

(event Collision|EventActorBeginOverlap
  (params (OtherActor :type Actor%20Object%20Reference)))

(event EventInteract
  (if (not (Variables|Default|GetisLocked))
    (Utilities|FlowControl|FlipFlop
      (:A
        (Variables|Default|SetisClose false)
        (Audio|PlaySoundatLocation "/Game/Audio/openDoor.openDoor" "0, 0, 0" "0, 0, 0" 1.0 1.0 0.0 0 0 0 0)
        (bind _doortrack (Timeline|Timeline Play)
          (:Update
            (Transformation|SetRelativeRotation (Variables|Default|GetSM_Door) (Math|Rotator|MakeRotator 0.0 0.0 (Math|Float|Lerp 0.0 1.1e+02 _doortrack)) false false))))
      (:B
        (Variables|Default|SetisClose true)
        (Audio|PlaySoundatLocation "/Game/Audio/closeDoor.closeDoor" "0, 0, 0" "0, 0, 0" 1.0 1.0 0.0 0 0 0 0)
        (Timeline|Timeline Reverse)))))

(event EventTick
  (params (DeltaSeconds :type Float%20%28single-precision%29)))

(fn ConstructionScript)